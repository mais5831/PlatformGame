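; BP_MoveAlongSplinePlatform is a platform actor that travels along the spline of a BP_SplinePath actor, starting at BeginPlay.
; It grabs the path via GetActorOfClass, so it assumes a single path in the level.
; A timeline, with play rate scaled by TimeToComplete, lerps distance over the spline length to set the transform each update.
; Location is sampled in world space, but rotation in the spline's local space.
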(event `self.ReceiveBeginPlay`
  (bind _returnvalue (`GameplayStatics.GetActorOfClass` "/Game/Blueprints/BP_SplinePath.BP_SplinePath_C"))
  (set `self.Spline Ref` _returnvalue)
  (`self.Move Object`))

(event `Move Object`
  (`TimelineComponent.SetPlayRate` (`self.Move Object T`) (/ 1.0 (`self.TimeToComplete`)))
  (bind (_direction _move_track) (`Timeline|Move Object T`)
    (:`Update`
      (bind _returnvalue (`KismetMathLibrary.Lerp` 0.0 (`SplineComponent.GetSplineLength` (`/Game/Blueprints/BP_SplinePath.Spline` (`self.Spline Ref`))) _move_track))
      (`self.K2_SetActorTransform` (`KismetMathLibrary.MakeTransform` (`SplineComponent.GetLocationAtDistanceAlongSpline` (`/Game/Blueprints/BP_SplinePath.Spline` (`self.Spline Ref`)) _returnvalue "World") (`SplineComponent.GetRotationAtDistanceAlongSpline` (`/Game/Blueprints/BP_SplinePath.Spline` (`self.Spline Ref`)) _returnvalue "Local"))))))

(fn `UserConstructionScript`)