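; BP_Guild_Shopkeeper is an interactable shopkeeper that opens a shop screen for the player.
; Its ShopTrigger overlap shows or removes an interact prompt widget for BP_Player.
; Interact briefly flags the prompt as pressed, then removes it and blends the camera to the shopkeeper.
; After the blend it opens Shopkeeper_UI with UI-only input and cursor, hides the player character and stops active movement.
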(event `self.ShopTrigger.OnComponentBeginOverlap`
  (params (OverlappedComponent :type "PrimitiveComponent Object Reference") (OtherActor :type "Actor Object Reference") (OtherComp :type "PrimitiveComponent Object Reference") (OtherBodyIndex :type Integer) (bFromSweep :type Boolean) (SweepResult :type "HitResult Structure (by ref)"))
  ;[0 0 0 1 32] Interact Button Popup
  (cast `/Game/Blueprints/BP_Player` OtherActor)
  (bind _returnvalue (`|CreateWidget` "/Game/Blueprints/Interact_Prompt_Widget.Interact_Prompt_Widget_C"))
  (`UserWidget.AddToViewport` _returnvalue 0))

(event `self.ShopTrigger.OnComponentEndOverlap`
  (params (OverlappedComponent :type "PrimitiveComponent Object Reference") (OtherActor :type "Actor Object Reference") (OtherComp :type "PrimitiveComponent Object Reference") (OtherBodyIndex :type Integer))
  ;[0 0 0 1 32] Interact Button Popup
  (cast `/Game/Blueprints/BP_Player` OtherActor)
  (`Widget.RemoveFromParent` (stale `self.ShopTrigger.OnComponentBeginOverlap` _returnvalue)))

(event `/Game/Blueprints/BP_Interact_Interface.Interact`
  (bind _returnvalue (`GameplayStatics.GetPlayerController` 0))
  (bind _returnvalue_2 (`GameplayStatics.GetPlayerCharacter` 0))
  (set `/Game/Blueprints/Interact_Prompt_Widget.IsPressed` true (stale `self.ShopTrigger.OnComponentBeginOverlap` _returnvalue))
  (`KismetSystemLibrary.Delay` 0.2)
  (set `/Game/Blueprints/Interact_Prompt_Widget.IsPressed` false (stale `self.ShopTrigger.OnComponentBeginOverlap` _returnvalue))
  (cast `/Game/Blueprints/BP_Player` (stale `self.ShopTrigger.OnComponentBeginOverlap` OtherActor))
  (`Widget.RemoveFromParent` (stale `self.ShopTrigger.OnComponentBeginOverlap` _returnvalue))
  (`PlayerController.SetViewTargetWithBlend` (`GameplayStatics.GetPlayerController` 0) self 1.0 "VTBlend_Linear" 0.0 false)
  (`KismetSystemLibrary.Delay` 1.0)
  (bind _returnvalue_3 (`|CreateWidget` "/Game/HUD/Shopkeeper_UI.Shopkeeper_UI_C" null self null))
  (`UserWidget.AddToViewport` _returnvalue_3 0)
  (`WidgetBlueprintLibrary.SetInputMode_UIOnlyEx` _returnvalue _returnvalue_3)
  (set `PlayerController.bShowMouseCursor` true _returnvalue)
  (`self.SetActorHiddenInGame` _returnvalue_2 true)
  (`NavMovementComponent.StopActiveMovement` (`Character.CharacterMovement` _returnvalue_2)))

(fn `UserConstructionScript`)