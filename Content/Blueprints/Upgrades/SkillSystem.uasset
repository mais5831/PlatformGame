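; SkillSystem tracks the skills that have been unlocked and the tier of each.
; It stores them in an UnlockedSkills map keyed by row name, with the tier as the value.
; AddSkill inserts a new skill at tier one or raises an existing one by a tier, with no upper limit, and always returns true.
; QuerySkill reports whether a skill is unlocked and at which tier.
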(fn `Add Skill`
  (params (RowName :type String))
  (returns (WasSuccessful :type Boolean))
  (bind _rowname (`local.RowName`))
  (bind (_value _returnvalue) (`BlueprintMapLibrary.Map_Find` (`self.UnlockedSkills`) RowName))
  ;[1 1 1] Add Skill or add 1 to tier if skill already unlocked.
  (if _returnvalue
    (`BlueprintMapLibrary.Map_Add` (`self.UnlockedSkills`) _rowname (+ _value 1))
    (return true)
    (else
      (`BlueprintMapLibrary.Map_Add` (`self.UnlockedSkills`) _rowname 1)
      (return true))))

(fn `Query Skill`
  (params (RowName :type String))
  (returns (IsSuccessful :type Boolean) (Tier :type Integer))
  (bind (_value _returnvalue) (`BlueprintMapLibrary.Map_Find` (`self.UnlockedSkills`) RowName))
  ;[1 1 1] Checks if skill is unlocked
  (if _returnvalue
    (return true _value)
    (else
      (return false _value))))