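; Goblin enemy Blueprint that chases and attacks the player while they are within overlap range.
; Beginning overlap with BP_Player starts an AI MoveTo toward the player, and ending overlap clears the range flag and stops movement.
; On arrival it plays an attack montage gated by an AttackRate cooldown, re-chasing when the montage completes if still in range, or immediately while on cooldown.
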(event `self.ReceiveActorBeginOverlap`
  (params (OtherActor :type "Actor Object Reference"))
  ;[1 1 1] When Player is Near Enemy begins Chase Player
  (bind _asbp_player (cast `/Game/Blueprints/BP_Player` OtherActor))
  (set `/Game/Blueprints/BP_Player.PlayerRef` _asbp_player _asbp_player)
  (set `self.Player In Range` true)
  (`self.Chase The Player`))

(event `self.ReceiveActorEndOverlap`
  (params (OtherActor :type "Actor Object Reference"))
  ;[1 1 1] If Player is not in range, Enemy stops chase
  (cast `/Game/Blueprints/BP_Player` OtherActor)
  (set `self.Player In Range` false)
  (`MovementComponent.StopMovementImmediately` (`self.CharacterMovement`)))

(event `Chase The Player`
  (`|AIMoveTo` self (0.0 0.0 0.0) (`GameplayStatics.GetPlayerCharacter` 0) 100.0
    (:`OnSuccess`
      (if (`self.Can Attack`)
        (set `self.Can Attack` false)
        (`|PlayMontage` (`self.Mesh`) "/Game/Assets/Goblin_Male/Attack.Attack"
          (:`then`
            (`KismetSystemLibrary.Delay` (`self.Attack Rate`))
            (set `self.Can Attack` true))
          (:`OnCompleted`
            (if (`self.Player In Range`)
              (`self.Chase The Player`))))
        (else
          (`self.Chase The Player`))))))

(fn `UserConstructionScript`)